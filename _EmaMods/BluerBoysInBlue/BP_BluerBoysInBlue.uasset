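; Mod actor that gives the "Boys in Blue" heist a bluer look by changing the color temperature of its sunlight.
; On BeginPlay it compares the heist display name from the SBZ mission state against that title.
; On a match, it takes the first DirectionalLight in the level and sets its light component to a fixed temperature.
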(event EventBeginPlay
  (if (Utilities|Enum|Equal(Enum) (Variables|/Script/Starbreeze.PD3HeistDataAsset|GetHeistDisplayName (Variables|/Script/Starbreeze.SBZMissionState|GetCurrentHeistData (Class|SBZMissionState|GetSBZMissionState))) (Utilities|Text|ToText(String) "Boys in Blue"))
    (bind _outactors (Actor|GetAllActorsOfClass "/Script/Engine.DirectionalLight"))
    (Class|LightComponent|SetTemperature (Variables|/Script/Engine.Light|GetLightComponent (Utilities|Array|Get(acopy) _outactors)) 6.5e+03)))

(fn ConstructionScript
  (|CallParentFunction))